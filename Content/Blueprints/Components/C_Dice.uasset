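; C_Dice is a dice component that rolls random faces and keeps a history of the results.
; RollDice picks a random entry from DiceFaces, appends it to LastResults and returns it.
; TenLastResults is a debug printout that loops over a fixed range at the start of that never-trimmed history, so it shows neither ten entries nor the most recent ones.
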(event EventBeginPlay)

(event EventTick
  (params (DeltaSeconds :type Float%20%28single-precision%29)))

(fn RollDice
  (bind _output_get (LocalVariables|SetRollResult (.OutItem (Utilities|Array|Random (Variables|Default|GetDiceFaces)))))
  (Utilities|Array|Add (Variables|Default|GetLastResults) _output_get)
  (return _output_get))

(fn TenLastResults
  (LocalVariables|SetParcoursLastResult 0)
  (if (< (LocalVariables|GetParcoursLastResult) 9) :!label _label
    (bind _result (Math|Integer|IncrementInt (LocalVariables|GetParcoursLastResult))
      (:%20%20
        (Development|PrintString (Utilities|String|Append "Result " (Utilities|String|ToString(Integer) _result) " : " (Utilities|String|EnumtoString (Utilities|Array|Get(acopy) (Variables|Default|GetLastResults) (LocalVariables|GetParcoursLastResult)))))
        (goto _label)))))