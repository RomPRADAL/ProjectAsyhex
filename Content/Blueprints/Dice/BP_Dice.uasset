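; Six-sided dice actor with combat-themed results (Melee, Defence, Power, Reload, Ranged, Wind), driven by its CDice component.
; Initialisation looks up each CDice face in DT_Dice and applies its material to the matching face mesh.
; RotateDiceToValue turns the Pivot instantly per result, offsetting its current relative roll or pitch and setting that as world rotation.
; BeginPlay also runs TestDice, which rolls, rotates and prints ten times, then calls TenLastResults.
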(event EventBeginPlay
  (CallFunction|Initialisation)
  (CallFunction|TestDice))

(event EventTick
  (params (DeltaSeconds :type Float%20%28single-precision%29)))

(fn ConstructionScript)

(fn Initialisation
  (for (_array_element _array_index) (Variables|/Game/Blueprints/Components/C_Dice.C_Dice_C|GetDiceFaces (Variables|Default|GetC_Dice))
    (bind _returnvalue (Utilities|GetDataTableRow "/Game/Blueprints/Database/DT_Dice.DT_Dice" (Utilities|String|StringToName (Utilities|String|EnumtoString _array_element)))
      (:then
        (switch int _array_index
          (:0
            (Rendering|Material|SetMaterial (Variables|Default|GetFace) 0 (.facematerial _returnvalue)))
          (:1
            (Rendering|Material|SetMaterial (Variables|Default|GetFace1) 0 (.facematerial _returnvalue)))
          (:2
            (Rendering|Material|SetMaterial (Variables|Default|GetFace2) 0 (.facematerial _returnvalue)))
          (:3
            (Rendering|Material|SetMaterial (Variables|Default|GetFace3) 0 (.facematerial _returnvalue)))
          (:4
            (Rendering|Material|SetMaterial (Variables|Default|GetFace4) 0 (.facematerial _returnvalue)))
          (:5
            (Rendering|Material|SetMaterial (Variables|Default|GetFace5) 0 (.facematerial _returnvalue))))))))

(fn TestDice
  (while (< (LocalVariables|GetI) 10)
    (bind _result (Default|RollDice (Variables|Default|GetC_Dice)))
    (CallFunction|RotateDicetoValue _result)
    (Math|Integer|IncrementInt (LocalVariables|GetI)
      (:%20%20
        (Development|PrintString (Utilities|String|Append "Roll numéro " (Utilities|String|ToString(Integer) (LocalVariables|GetI)) " : " (Utilities|String|EnumtoString _result))))))
  (Default|TenLastResults (Variables|Default|GetC_Dice)))

(fn RotateDicetoValue
  (params (Result :type E_DiceFaces%20Enum :default "NewEnumerator0"))
  (bind _pivot (Variables|Default|GetPivot))
  (bind _pivot_2 (Variables|Default|GetPivot))
  (bind _pivot_3 (Variables|Default|GetPivot))
  (bind _pivot_4 (Variables|Default|GetPivot))
  (bind _pivot_5 (Variables|Default|GetPivot))
  (bind _pivot_6 (Variables|Default|GetPivot))
  (switch Utilities|FlowControl|Switch|SwitchonE_DiceFaces Result
    (:NewEnumerator0
      (Transformation|SetWorldRotation _pivot_4 (Math|Rotator|MakeRotator (+ (.roll (Variables|/Script/Engine.SceneComponent|GetRelativeRotation _pivot_4)) 9e+01) 0.0 0.0) false false))
    (:NewEnumerator1
      (Transformation|SetWorldRotation _pivot_5 (Math|Rotator|MakeRotator (+ (.roll (Variables|/Script/Engine.SceneComponent|GetRelativeRotation _pivot_5)) -9e+01) 0.0 0.0) false false))
    (:NewEnumerator2
      (Transformation|SetWorldRotation _pivot_6 (Math|Rotator|MakeRotator (+ (.roll (Variables|/Script/Engine.SceneComponent|GetRelativeRotation _pivot_6)) 1.8e+02) 0.0 0.0) false false))
    (:NewEnumerator3
      (Transformation|SetWorldRotation _pivot_2 (Math|Rotator|MakeRotator (+ (.roll (Variables|/Script/Engine.SceneComponent|GetRelativeRotation _pivot_2)) 0.0) 0.0 0.0) false false))
    (:NewEnumerator4
      (Transformation|SetWorldRotation _pivot_3 (Math|Rotator|MakeRotator 0.0 (+ (.pitch (Variables|/Script/Engine.SceneComponent|GetRelativeRotation _pivot_3)) -9e+01) 0.0) false false))
    (:NewEnumerator5
      (Transformation|SetWorldRotation _pivot (Math|Rotator|MakeRotator 0.0 (+ (.pitch (Variables|/Script/Engine.SceneComponent|GetRelativeRotation _pivot)) 9e+01) 0.0) false false))))