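; BP_Hex is a hex grid cell Blueprint identified by horizontal and vertical coordinates.
; Initialisation builds HexName from both coordinates in a "Hex<H>-<V>" pattern, then calls MakeAdjacentHexs.
; MakeAdjacentHexs is an unfinished stub: its even/odd column check is disconnected, so it finds no neighbours.
; The event graph and construction script are empty, and nothing in this Blueprint calls Initialisation.
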(event EventBeginPlay)

(event Collision|EventActorBeginOverlap
  (params (OtherActor :type Actor%20Object%20Reference)))

(event EventTick
  (params (DeltaSeconds :type Float%20%28single-precision%29)))

(fn ConstructionScript)

(fn MakeAdjacentHexs)

(fn MakeName
  (Variables|Default|SetHexName (Utilities|String|Append "Hex " (Utilities|String|ToString(Integer) (Variables|Default|GetCoordHorizontal)) "-" (Utilities|String|ToString(Integer) (Variables|Default|GetCoordVertical)))))

(fn Initialisation
  (CallFunction|MakeName)
  (CallFunction|MakeAdjacentHexs))