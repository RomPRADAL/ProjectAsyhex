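; Game mode Blueprint that gathers and initializes the level's hex grid and looks hexes up by coordinates.
; On BeginPlay, InitGrid collects all BP_Hex actors, sets hex 0,0 as DefaultHex, tests another lookup, then initializes every hex.
; FindHex scans the unsorted array linearly, falling back to DefaultHex when nothing matches.
; SortAllHex, an insertion sort by horizontal then vertical coordinate with debug prints, is never called here.
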(event EventBeginPlay
  (Utilities|FlowControl|Sequence
    (:then_0
      (CallFunction|InitGrid))))

(fn ConstructionScript)

(fn FindHex
  (params (CoordHorizontal :type Integer) (CoordVertical :type Integer))
  (LocalVariables|SetFoundHex 0)
  (LocalVariables|SetParcoursFindHex 0)
  (if (< (LocalVariables|GetParcoursFindHex) (Utilities|Array|Length (Variables|Default|GetAllHexUnsorted))) :!label _label
    (if (and (== (Variables|/Game/Blueprints/Grid/BP_Hex.BP_Hex_C|GetCoordHorizontal (Utilities|Array|Get(acopy) (Variables|Default|GetAllHexUnsorted) (LocalVariables|GetParcoursFindHex))) CoordHorizontal) (== (Variables|/Game/Blueprints/Grid/BP_Hex.BP_Hex_C|GetCoordVertical (Utilities|Array|Get(acopy) (Variables|Default|GetAllHexUnsorted) (LocalVariables|GetParcoursFindHex))) CoordVertical))
      (LocalVariables|SetFoundHex (Utilities|Array|Get(acopy) (Variables|Default|GetAllHexUnsorted) (LocalVariables|GetParcoursFindHex)))
      (else
        (Math|Integer|IncrementInt (LocalVariables|GetParcoursFindHex)
          (:%20%20
            (goto _label)))))
    (else
      (LocalVariables|SetFoundHex (Variables|Default|GetDefaultHex))))
  (return (LocalVariables|GetFoundHex) (LocalVariables|GetParcoursFindHex)))

(fn SortAllHex
  (bind _allhexsorted (Variables|Default|GetAllHexSorted))
  (bind _allhexsorted_2 (Variables|Default|GetAllHexSorted))
  (bind _output (Utilities|Array|Get(acopy) _allhexsorted_2))
  (LocalVariables|SetParcoursUnsorted 0)
  (LocalVariables|SetLengthUnsorted (Utilities|Array|Length (Variables|Default|GetAllHexUnsorted)))
  (Utilities|Array|Resize _allhexsorted (LocalVariables|GetLengthUnsorted))
  (Development|PrintString (Utilities|String|Append "Taille AllHexUnsorted : " (Utilities|String|ToString(Integer) (Utilities|Array|Length (Variables|Default|GetAllHexUnsorted)))))
  (Development|PrintString (Utilities|String|Append "Taille AllHexSorted : " (Utilities|String|ToString(Integer) (Utilities|Array|Length _allhexsorted))))
  ;[0 0.0615 1] On met le premier élément, quel qu'il soit, a l'index 0
  (Utilities|Array|Insert (Variables|Default|GetAllHexSorted) (Utilities|Array|Get(acopy) (Variables|Default|GetAllHexUnsorted)))
  (Math|Integer|IncrementInt (LocalVariables|GetParcoursUnsorted)
    (:%20%20
      (if (< (LocalVariables|GetParcoursUnsorted) (LocalVariables|GetLengthUnsorted)) :!label _label
        (LocalVariables|SetParcoursSorted 0)
        (if (< (Variables|/Game/Blueprints/Grid/BP_Hex.BP_Hex_C|GetCoordHorizontal (Utilities|Array|Get(acopy) (Variables|Default|GetAllHexUnsorted) (LocalVariables|GetParcoursUnsorted))) (Variables|/Game/Blueprints/Grid/BP_Hex.BP_Hex_C|GetCoordHorizontal (Utilities|Array|Get(acopy) (Variables|Default|GetAllHexSorted) (LocalVariables|GetParcoursSorted))))
          (Utilities|Array|Insert (Variables|Default|GetAllHexSorted) (Utilities|Array|Get(acopy) (Variables|Default|GetAllHexUnsorted) (LocalVariables|GetParcoursUnsorted)) (LocalVariables|GetParcoursSorted))
          (Math|Integer|IncrementInt (LocalVariables|GetParcoursUnsorted)
            (:%20%20
              (goto _label)))
          (else
            (Utilities|IsValid (Utilities|Array|Get(acopy) (Variables|Default|GetAllHexSorted) (LocalVariables|GetParcoursSorted))
              (:Is%20Valid
                (if (> (Variables|/Game/Blueprints/Grid/BP_Hex.BP_Hex_C|GetCoordHorizontal (Utilities|Array|Get(acopy) (Variables|Default|GetAllHexUnsorted) (LocalVariables|GetParcoursUnsorted))) (Variables|/Game/Blueprints/Grid/BP_Hex.BP_Hex_C|GetCoordHorizontal (Utilities|Array|Get(acopy) (Variables|Default|GetAllHexSorted) (LocalVariables|GetParcoursSorted)))) :!label _label_2
                  (Math|Integer|IncrementInt (LocalVariables|GetParcoursSorted)
                    (:%20%20
                      (goto _label_2)))
                  (else
                    _)))
              (:Is%20Not%20Valid
                _))
            (if (== (Variables|/Game/Blueprints/Grid/BP_Hex.BP_Hex_C|GetCoordHorizontal (Utilities|Array|Get(acopy) (Variables|Default|GetAllHexUnsorted) (LocalVariables|GetParcoursUnsorted))) (Variables|/Game/Blueprints/Grid/BP_Hex.BP_Hex_C|GetCoordHorizontal (Utilities|Array|Get(acopy) (Variables|Default|GetAllHexSorted) (LocalVariables|GetParcoursSorted)))) :!label _label_3
              (if (< (Variables|/Game/Blueprints/Grid/BP_Hex.BP_Hex_C|GetCoordVertical (Utilities|Array|Get(acopy) (Variables|Default|GetAllHexUnsorted) (LocalVariables|GetParcoursUnsorted))) (Variables|/Game/Blueprints/Grid/BP_Hex.BP_Hex_C|GetCoordVertical (Utilities|Array|Get(acopy) (Variables|Default|GetAllHexSorted) (LocalVariables|GetParcoursSorted))))
                (Utilities|Array|Insert (Variables|Default|GetAllHexSorted) 0 (LocalVariables|GetParcoursSorted))
                (Math|Integer|IncrementInt (LocalVariables|GetParcoursUnsorted)
                  (:%20%20
                    (goto _label)))
                (elif (and (> (Variables|/Game/Blueprints/Grid/BP_Hex.BP_Hex_C|GetCoordVertical (Utilities|Array|Get(acopy) (Variables|Default|GetAllHexUnsorted) (LocalVariables|GetParcoursUnsorted))) (Variables|/Game/Blueprints/Grid/BP_Hex.BP_Hex_C|GetCoordVertical (Utilities|Array|Get(acopy) (Variables|Default|GetAllHexSorted) (LocalVariables|GetParcoursSorted)))) (Utilities|IsValid (Utilities|Array|Get(acopy) (Variables|Default|GetAllHexSorted) (LocalVariables|GetParcoursSorted))))
                  (Math|Integer|IncrementInt (LocalVariables|GetParcoursSorted)
                    (:%20%20
                      (goto _label_3)))
                  (else
                    (if (and (== (Variables|/Game/Blueprints/Grid/BP_Hex.BP_Hex_C|GetCoordVertical (Utilities|Array|Get(acopy) (Variables|Default|GetAllHexUnsorted) (LocalVariables|GetParcoursUnsorted))) (Variables|/Game/Blueprints/Grid/BP_Hex.BP_Hex_C|GetCoordVertical (Utilities|Array|Get(acopy) (Variables|Default|GetAllHexSorted) (LocalVariables|GetParcoursSorted)))) (Utilities|IsValid (Utilities|Array|Get(acopy) (Variables|Default|GetAllHexSorted) (LocalVariables|GetParcoursSorted))))
                      (Development|PrintString (Utilities|String|Append "Doublon : " (Utilities|String|ToString(Integer) (Variables|/Game/Blueprints/Grid/BP_Hex.BP_Hex_C|GetCoordVertical (Utilities|Array|Get(acopy) (Variables|Default|GetAllHexUnsorted) (LocalVariables|GetParcoursUnsorted)))) "-" (Utilities|String|ToString(Integer) (Variables|/Game/Blueprints/Grid/BP_Hex.BP_Hex_C|GetCoordVertical (Utilities|Array|Get(acopy) (Variables|Default|GetAllHexSorted) (LocalVariables|GetParcoursSorted))))))
                      (else
                        (Utilities|Array|Insert (Variables|Default|GetAllHexSorted) 0 (LocalVariables|GetParcoursSorted))))
                    (Math|Integer|IncrementInt (LocalVariables|GetParcoursUnsorted)
                      (:%20%20
                        (goto _label))))))
              (else
                (Utilities|Array|Insert (Variables|Default|GetAllHexSorted) 0 (LocalVariables|GetParcoursSorted))
                (Math|Integer|IncrementInt (LocalVariables|GetParcoursUnsorted)
                  (:%20%20
                    (goto _label)))))))
        (else
          (Development|PrintString "Finis rien a planté")
          (Default|Initialisation _output)
          (Development|PrintString (Utilities|String|Append "Premier élément : " (Variables|/Game/Blueprints/Grid/BP_Hex.BP_Hex_C|GetHexName _output))))))))

(fn InitGrid
  (Utilities|FlowControl|Sequence
    (:then_0
      (bind _outactors (Actor|GetAllActorsOfClass "/Game/Blueprints/Grid/BP_Hex.BP_Hex_C"))
      (Variables|Default|SetAllHexUnsorted _outactors)
      (Development|PrintString "AllHexUnsorted ok"))
    (:then_1
      (bind _hexfound (CallFunction|FindHex))
      (bind _output_get (Variables|Default|SetDefaultHex _hexfound))
      (Default|Initialisation _output_get)
      (Development|PrintString (Utilities|String|Append "Default Hex : " (Variables|/Game/Blueprints/Grid/BP_Hex.BP_Hex_C|GetHexName _output_get))))
    (:then_2
      (bind _hexfound_2 (CallFunction|FindHex 3 2))
      (Default|Initialisation _hexfound_2)
      (Development|PrintString (Utilities|String|Append "Test Hex : " (Variables|/Game/Blueprints/Grid/BP_Hex.BP_Hex_C|GetHexName _hexfound_2))))
    (:then_3
      (for _array_element (Variables|Default|GetAllHexUnsorted)
        (Default|Initialisation _array_element))
      (Development|PrintString "All Hexs Init"))))